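; BP_GameState is a game state that reacts to replicated flags for a tasseomancy (tea leaf reading) activity.
; When IsFinished replicates true, its RepNotify shows the end widget, hides the form sheet, calls UpdateTasseo on the game instance and resets the flag.
; The CleanTea RepNotify removes every added ingredient widget from the blank canvas widget on the cup.
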(fn `OnRep_CleanTea`
  (bind _aswbp_blank_canva (cast `/Game/Widget/WBP_BlankCanva` (`WidgetComponent.GetWidget` (`/Game/Blueprints/Tasseomancy/BP_Cup.Widget1` (`self.Cup`)))))
  (for _array_element (`/Game/Widget/WBP_BlankCanva.IngredientsAdded` _aswbp_blank_canva)
    (`Widget.RemoveFromParent` _array_element)))

(fn `OnRep_IsFinished`
  (if (`self.IsFinished`)
    (bind _returnvalue (`|CreateWidget` "/Game/Widget/Tasseomancy/WBP_EndTasseomancy.WBP_EndTasseomancy_C"))
    (`UserWidget.AddToViewport` _returnvalue 0)
    (`SceneComponent.SetVisibility` (`Actor.RootComponent` (`self.FormSheet`)) false true)
    (bind _asmain_game_instance (cast `/Game/Blueprints/MainGameInstance` (`GameplayStatics.GetGameInstance`)))
    (`/Game/Blueprints/MainGameInstance.UpdateTasseo` _asmain_game_instance)
    (set `self.IsFinished` false)))

(fn `UserConstructionScript`)