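; MainGameInstance is the game instance, holding per-visitor "Tasseo" visibility states for four visitors: Kiril, Grigor, Valeri and Anca.
; Its UpdateTasseo event switches on CurrentVisitor to pick that visitor's visibility array.
; It then sets the entry matching the one-based ChoiceSelected to Visible, recording the selected choice as revealed.
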(event `UpdateTasseo`
  (bind _returnvalue (- (`self.choiceSelected`) 1))
  (switch `int` (`self.CurrentVisitor`)
    (:`1`
      (`|VariableSetRef` (`|GetArrayItem` (`self.KirilTasseoVisibilityState`) _returnvalue) "Visible"))
    (:`2`
      (`|VariableSetRef` (`|GetArrayItem` (`self.GrigorTasseoVisibilityState`) _returnvalue) "Visible"))
    (:`3`
      (`|VariableSetRef` (`|GetArrayItem` (`self.ValeriTasseoVisibilityState`) _returnvalue) "Visible"))
    (:`4`
      (`|VariableSetRef` (`|GetArrayItem` (`self.AncaTasseoVisibilityState`) _returnvalue) "Visible"))))