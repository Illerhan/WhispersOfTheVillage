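; BP_Cup is the tasseomancy cup actor, which displays feedback for a win and for individual symbols.
; On BeginPlay it registers itself as the Cup on BP_GameState and creates a dynamic material instance for its Halo.
; WinFeedback activates Niagara particles and reveals the Halo, with the Highlight timeline driving its opacity.
; IndividualSymbolFeedback resets a second Niagara effect's relative location, then plays a validation sound and activates that effect.
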(event `self.ReceiveBeginPlay`
  (bind _halo (`self.Halo`))
  (`SceneComponent.SetVisibility` (`self.Widget1`) false false)
  (`SceneComponent.SetVisibility` (`self.Widget1`) true false)
  (bind _asbp_game_state (cast `/Game/Blueprints/BP_GameState` (`GameplayStatics.GetGameState`)))
  (set `/Game/Blueprints/BP_GameState.Cup` self _asbp_game_state)
  (bind _returnvalue (`PrimitiveComponent.CreateDynamicMaterialInstance` _halo 0 (`PrimitiveComponent.GetMaterial` _halo 0) "None"))
  (bind _output_get (set `self.HaloMat` _returnvalue))
  (`PrimitiveComponent.SetMaterial` (`self.Halo`) 0 _output_get))

(event `WinFeedback`
  (`ActorComponent.Activate` (`self.Niagara`) false)
  (`SceneComponent.SetVisibility` (`self.Halo`) true false)
  (bind (_direction _highlight) (`Timeline|Highlight`)
    (:`Update`
      (`MaterialInstanceDynamic.SetScalarParameterValue` (`self.HaloMat`) "Opacity" _highlight))))

(event `IndividualSymbolFeedback`
  (bind _niagara_individualsymbols (`self.Niagara_IndividualSymbols`))
  (`SceneComponent.K2_SetRelativeLocation` _niagara_individualsymbols (0.0 0.0 0.0) false false)
  (`GameplayStatics.PlaySound2D` "/Game/Sounds/Sound_Cue/ValidationTasseomancy/A_ValidationForm_01_Cue.A_ValidationForm_01_Cue" 1.0 1.0 0.0 null null)
  (`ActorComponent.Activate` _niagara_individualsymbols false))

(fn `UserConstructionScript`)