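; Player controller that handles dialogue advancing, the pause menu and the notebook's open and close feedback.
; Left click advances the HUD_Dialogue widget on the cached BP_Dialogue actor, only in L_Dialog_Clean with no menu open.
; L opens the pause menu, flags IsMenuOpen on BP_PlayerState and pauses the game.
; The BookOpen RepNotify plays sounds, creates the book widget on opening and toggles dialogue pausing.
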(event `self.ReceiveBeginPlay`
  (bind _returnvalue (`GameplayStatics.GetActorOfClass` "/Game/Blueprints/BP_Dialogue.BP_Dialogue_C"))
  (set `self.DialWidget` _returnvalue))

(event `Key|LeftMouseButton`
  (params (Key :type "Key Structure"))
  (bind _returnvalue (`WidgetComponent.GetWidget` (`/Game/Blueprints/BP_Dialogue.WidgetDialogue` (`self.DialWidget`))))
  (:`Pressed`
    (if (not (`/Game/Blueprints/BP_PlayerState.IsMenuOpen` (cast `/Game/Blueprints/BP_PlayerState` (`self.PlayerState`) :!pure true)))
      (bind _returnvalue_2 (`GameplayStatics.GetCurrentLevelName` true))
      (if (`KismetStringLibrary.EqualEqual_StrStr` _returnvalue_2 "L_Dialog_Clean")
        (`/Engine/EditorBlueprintResources/StandardMacros.IsValid` _returnvalue
          (:`Is Valid`
            (bind _ashud_dialogue (cast `/Game/Widget/HUD_Dialogue` _returnvalue))
            (`/Game/Widget/HUD_Dialogue.GoToNextDialogue` _ashud_dialogue)))))))

(event `Key|L`
  (params (Key :type "Key Structure"))
  (:`Pressed`
    (bind _returnvalue (`|CreateWidget` "/Game/Widget/WBP_PauseMenu.WBP_PauseMenu_C"))
    (`UserWidget.AddToViewport` _returnvalue 0)
    (bind _asbp_player_state (cast `/Game/Blueprints/BP_PlayerState` (`self.PlayerState`)))
    (set `/Game/Blueprints/BP_PlayerState.IsMenuOpen` true _asbp_player_state)
    (`GameplayStatics.SetGamePaused` true)))

(fn `OnRep_BookOpen`
  (if (`self.BookOpen`)
    (`GameplayStatics.PlaySound2D` "/Game/Sounds/Sound_Cue/OpenNoteBook/A_OpenNoteBook_01_Cue.A_OpenNoteBook_01_Cue" 1.0 1.0 0.0 null null)
    (bind _returnvalue (`|CreateWidget` "/Game/Widget/WBP_Book.WBP_Book_C"))
    (`UserWidget.AddToViewport` _returnvalue 0)
    (bind _foundwidgets (`WidgetBlueprintLibrary.GetAllWidgetsOfClass` "/Game/Widget/HUD_Dialogue.HUD_Dialogue_C" false))
    (set `/Game/Widget/HUD_Dialogue.IsPaused` true (`|GetArrayItem` _foundwidgets))
    (else
      (`GameplayStatics.PlaySound2D` "/Game/Sounds/Sound_Cue/CloseNoteBook/A_CloseNoteBook_01_Cue.A_CloseNoteBook_01_Cue" 1.0 1.0 0.0 null null)
      (bind _foundwidgets_2 (`WidgetBlueprintLibrary.GetAllWidgetsOfClass` "/Game/Widget/HUD_Dialogue.HUD_Dialogue_C" false))
      (set `/Game/Widget/HUD_Dialogue.IsPaused` false (`|GetArrayItem` _foundwidgets_2)))))

(fn `UserConstructionScript`)