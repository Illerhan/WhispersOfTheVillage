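; Clickable tea ingredients actor that opens a UI widget when its static mesh is clicked.
; BeginPlay enables click events on the first player controller.
; The mesh's OnClicked creates the widget, places it at the mouse position with a small up-left offset, and adds it to the viewport.
; A ClickedOn function repeats the same spawning logic but is not called within this Blueprint.
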(event `self.ReceiveBeginPlay`
  (set `PlayerController.bEnableClickEvents` true (`GameplayStatics.GetPlayerController` 0)))

(event `self.StaticMesh.OnClicked`
  (params (TouchedComponent :type "PrimitiveComponent Object Reference") (ButtonPressed :type "Key Structure"))
  (bind _returnvalue (`|CreateWidget` (`self.Class`) null null null null))
  (bind _returnvalue_2 (`WidgetLayoutLibrary.GetMousePositionOnViewport`))
  (`UserWidget.SetPositionInViewport` _returnvalue (- _returnvalue_2 (50.0 50.0)) false)
  (`UserWidget.AddToViewport` _returnvalue 0))

(fn `ClickedOn`
  (bind _returnvalue (`|CreateWidget` (`self.Class`) null null null null))
  (bind _returnvalue_2 (`WidgetLayoutLibrary.GetMousePositionOnViewport`))
  (`UserWidget.SetPositionInViewport` _returnvalue (- _returnvalue_2 (50.0 50.0)) false)
  (`UserWidget.AddToViewport` _returnvalue 0))

(fn `UserConstructionScript`)