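; BP_FormSheet is an actor that shows a form list widget with next and previous navigation buttons.
; On BeginPlay it passes its Column value into the WBP_FormList_Old widget and binds the Next and Previous click events of the WBP_NextList button widget.
; Those events set the matching Next or Previous flag on GM_GameMode, leaving the page change to be handled elsewhere.
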(event `Next`
  (bind _asgm_game_mode (cast `/Game/Blueprints/GM_GameMode` (`GameplayStatics.GetGameMode`)))
  (set `/Game/Blueprints/GM_GameMode.Next` true _asgm_game_mode))

(event `Previous`
  (bind _asgm_game_mode (cast `/Game/Blueprints/GM_GameMode` (`GameplayStatics.GetGameMode`)))
  (set `/Game/Blueprints/GM_GameMode.Previous` true _asgm_game_mode))

(event `self.ReceiveBeginPlay`
  (bind _aswbp_next_list (cast `/Game/Widget/Old/WBP_NextList` (`WidgetComponent.GetWidget` (`self.Button`)) :!pure true))
  (bind _aswbp_form_list_old (cast `/Game/Widget/Old/WBP_FormList_Old` (`WidgetComponent.GetUserWidgetObject` (`self.Form`))))
  (set `/Game/Widget/Old/WBP_FormList_Old.Columns` (`self.Column`) _aswbp_form_list_old)
  (add `/Game/Widget/Old/WBP_NextList.PreviousClicked` _aswbp_next_list (delegate `Previous`))
  (add `/Game/Widget/Old/WBP_NextList.NextClicked` _aswbp_next_list (delegate `Next`)))

(fn `UserConstructionScript`)