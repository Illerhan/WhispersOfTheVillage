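; BP_Book is a clickable book actor that tells the player controller to open the book when clicked.
; On BeginPlay it creates a dynamic material on the cube's second slot to drive a highlight parameter.
; A timeline animates that highlight on day one with the first visitor until the book is clicked.
; After that first click, a second timeline fades the highlight in and out on cursor hover.
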(event `self.ReceiveBeginPlay`
  (bind _asmain_game_instance (cast `/Game/Blueprints/MainGameInstance` (`GameplayStatics.GetGameInstance`) :!pure true))
  (bind _asbp_player_controller (cast `/Game/Blueprints/BP_PlayerController` (`GameplayStatics.GetPlayerController` 0)))
  (set `self.As BP Player Controller` _asbp_player_controller)
  ;[1 1 1] Create Material to be able to use highlight
  (bind _returnvalue (`KismetMaterialLibrary.CreateDynamicMaterialInstance` (`PrimitiveComponent.GetMaterial` (`self.Cube`) 1)))
  (bind _output_get (set `self.DynamicMaterial` _returnvalue))
  (`PrimitiveComponent.SetMaterial` (`self.Cube`) 1 _output_get)
  (if (and (== (`/Game/Blueprints/MainGameInstance.CurrentVisitor` _asmain_game_instance) 1) (== (`/Game/Blueprints/MainGameInstance.CurrentlDay` _asmain_game_instance) 1))
    (bind (_direction _highlight) (`Timeline|Timeline` :!label _label)
      (:`Update`
        (`MaterialInstanceDynamic.SetScalarParameterValue` (`self.DynamicMaterial`) (`self.HighlightParameter`) _highlight)))))

(event `self.ReceiveTick`
  (params (DeltaSeconds :type "Float (single-precision)")))

(event `self.Cube.OnClicked`
  (params (TouchedComponent :type "PrimitiveComponent Object Reference") (ButtonPressed :type "Key Structure"))
  ;[1 1 1] Remplacer par un bool de MainGameInstance
  (set `self.HasClickedOnBook` true)
  (set `/Game/Blueprints/BP_PlayerController.BookOpen` true (`self.As BP Player Controller`))
  (goto _label :!via `Stop`))

(event `self.Cube.OnBeginCursorOver`
  (params (TouchedComponent :type "PrimitiveComponent Object Reference"))
  ;[1 1 1] Remplacer par un bool de MainGameInstance
  (if (`self.HasClickedOnBook`)
    (bind (_direction _highlight) (`Timeline|Highlight` :!label _label_2)
      (:`Update`
        (`MaterialInstanceDynamic.SetScalarParameterValue` (`self.DynamicMaterial`) (`self.HighlightParameter`) _highlight)))))

(event `self.Cube.OnEndCursorOver`
  (params (TouchedComponent :type "PrimitiveComponent Object Reference"))
  (goto _label_2 :!via `Reverse`))

(fn `UserConstructionScript`)